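; BP_HankCharacter is the Paper2D Hank character Blueprint, tracking lives and collected coins.
; LoseLife decrements Lives and calls Die once none remain.
; Die swaps the flipbook to a corpse, sets the Dead flag, stops movement and shows the end screen through its UI reference.
; PickupCoin increments the coin count.
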(fn ConstructionScript)

(fn LoseLife
  (bind _result (Math|Integer|DecrementInt (Variables|Default|GetLives))
    (:%20%20
      (bind _output_get (Variables|Default|SetLives _result))
      (if (<= _output_get 0)
        (CallFunction|Die)
        (else
          (return))))))

(fn Die
  (Sprite|SetFlipbook (Variables|Default|GetPaperFlipbook) "/Game/Textures/Player/Corpse.Corpse")
  (Variables|Default|SetDead true)
  (Class|HankCharacter|StopMoving)
  (Default|ShowEndScreen (Variables|Default|GetUIRef)))

(fn PickupCoin
  (bind _result (Math|Integer|IncrementInt (Variables|Default|GetCoins))
    (:%20%20
      (Variables|Default|SetCoins _result)
      (return))))