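; Base tile Blueprint for a lane-based game, designed to fill three spawn areas (left, middle, right) with obstacles and coins.
; PopulateTile randomly picks two different lanes and calls SpawnObstacle for each; separate logic finds the free lane for a coin row.
; Much is unwired: BeginPlay and end-of-tile overlap do nothing, both spawn functions create no actors, and the coin-lane logic is never reached.
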(event OnComponentBeginOverlap(EndOfTile)
  (params (OverlappedComponent :type Primitive%20Component%20Object%20Reference) (OtherActor :type Actor%20Object%20Reference) (OtherComp :type Primitive%20Component%20Object%20Reference) (OtherBodyIndex :type Integer) (bFromSweep :type Boolean) (SweepResult :type Hit%20Result%20Structure%20%28by%20ref%29)))

(event EventBeginPlay)

(fn ConstructionScript)

(fn SpawnObstacle
  (params (Spawn%20Transform :type Transform)))

(fn SpawnCoinRow
  (params (SpawnTransform :type Transform))
  (for _index (range 1 (Math|Random|RandomIntegerinRange 3 5))
    _)
  (return))

(fn PopulateTile
  (bind _output_get (LocalVariables|SetSampleInt1 (Math|Random|RandomIntegerinRange 0 2)))
  (switch int _output_get
    (:0
      (LocalVariables|SetSampleInt2 (Math|Random|RandomIntegerinRange 1 2)))
    (:1
      (LocalVariables|SetSampleInt2 (CallFunction|ReturnRandomValueOutOf2 0 2)))
    (:2
      (LocalVariables|SetSampleInt2 (Math|Random|RandomIntegerinRange 0 1))))
  ;[1 1 1] Spawn First Obstacle
  (switch int (LocalVariables|GetSampleInt1)
    (:0
      (CallFunction|SpawnObstacle (Math|Conversions|ToTransform(Vector) (Transformation|GetWorldLocation (Variables|Default|GetSpawnAreaLeft)))))
    (:1
      (CallFunction|SpawnObstacle (Math|Conversions|ToTransform(Vector) (Transformation|GetWorldLocation (Variables|Default|GetSpawnAreaMiddle)))))
    (:2
      (CallFunction|SpawnObstacle (Math|Conversions|ToTransform(Vector) (Transformation|GetWorldLocation (Variables|Default|GetSpawnAreaRight))))))
  ;[1 1 1] Spawn Second Obstacle
  (switch int (LocalVariables|GetSampleInt2)
    (:0
      (CallFunction|SpawnObstacle (Math|Conversions|ToTransform(Vector) (Transformation|GetWorldLocation (Variables|Default|GetSpawnAreaLeft)))))
    (:1
      (CallFunction|SpawnObstacle (Math|Conversions|ToTransform(Vector) (Transformation|GetWorldLocation (Variables|Default|GetSpawnAreaMiddle)))))
    (:2
      (CallFunction|SpawnObstacle (Math|Conversions|ToTransform(Vector) (Transformation|GetWorldLocation (Variables|Default|GetSpawnAreaRight))))))
  (Utilities|Casting|CastToHankGameMode (Game|GetGameMode)))

(fn ReturnRandomValueOutOf2
  (params (Value1 :type Integer) (Value2 :type Integer))
  (if (Math|Random|RandomBool)
    (return Value1)
    (else
      (return Value2))))